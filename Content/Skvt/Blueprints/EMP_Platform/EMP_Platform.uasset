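; EMP platform Blueprint that sends an EMP message to nearby electric actors.
; When something overlaps its Sphere, it draws a debug sphere and calls ApplyEMPMessage on overlapping actors implementing BPI_Eletric, deactivating DefaultSceneRoot after each call.
; A separate ToggleON function relays an on/off state to every entry in the Eletric array via ToggleOnMessage.
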(event `self.ReceiveBeginPlay`)

(event `self.Sphere.OnComponentBeginOverlap`
  (params (OverlappedComponent :type "PrimitiveComponent Object Reference") (OtherActor :type "Actor Object Reference") (OtherComp :type "PrimitiveComponent Object Reference") (OtherBodyIndex :type Integer) (bFromSweep :type Boolean) (SweepResult :type "HitResult Structure (by ref)"))
  (`KismetSystemLibrary.DrawDebugSphere` (0.0 0.0 0.0))
  (for _array_element (`PrimitiveComponent.GetOverlappingActors` (`self.Sphere`) "/Script/Engine.Actor")
    (bind _asbpi_eletric (cast `/Game/Skvt/Blueprints/BPI_Eletric` _array_element))
    (message `/Game/Skvt/Blueprints/BPI_Eletric.ApplyEMP` (`KismetSystemLibrary.Conv_InterfaceToObject` _asbpi_eletric))
    (`ActorComponent.Deactivate` (`self.DefaultSceneRoot`))))

(fn `ToggleON`
  (params (IsOn :type Boolean))
  (for _array_element (`self.Eletric`)
    (message `/Game/Skvt/Blueprints/BPI_Eletric.ToggleOn` _array_element IsOn)))

(fn `UserConstructionScript`)