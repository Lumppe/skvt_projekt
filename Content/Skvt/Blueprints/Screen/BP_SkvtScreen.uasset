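; BP_SkvtScreen is an in-world screen that displays a WBP_SkvtWeb widget through its Webpage component and can be toggled or disabled by an EMP.
; On BeginPlay it caches the cast widget as WebpageRef.
; Toggleon sets the component's visibility.
; ApplyEMP plays sparks and sound, then sets the component visible only in scene captures, with no restore in this graph.
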(event `self.ReceiveBeginPlay`
  (`self.Initialize`))

(event `/Game/Skvt/Blueprints/BPI_Eletric.ToggleOn`
  (params (IsOn :type Boolean))
  (`SceneComponent.SetVisibility` (`self.Webpage`) IsOn false))

(event `/Game/Skvt/Blueprints/BPI_Eletric.ApplyEMP`
  (`GameplayStatics.SpawnEmitterAttached` "/Game/StarterContent/Particles/P_Sparks.P_Sparks" (`self.Webpage`))
  (`GameplayStatics.PlaySoundAtLocation` "/Game/StarterContent/Audio/Fire_Sparks01_Cue.Fire_Sparks01_Cue" (0.0 0.0 0.0) (struct) 0.5 1.0 0.0 null null null null)
  (`PrimitiveComponent.SetVisibleInSceneCaptureOnly` (`self.Webpage`) true))

(fn `Initialize`
  (bind _aswbp_skvt_web (cast `/Game/Skvt/Blueprints/Screen/WBP_SkvtWeb` (`WidgetComponent.GetWidget` (`self.Webpage`))))
  (set `self.WebpageRef` _aswbp_skvt_web))

(fn `UserConstructionScript`)