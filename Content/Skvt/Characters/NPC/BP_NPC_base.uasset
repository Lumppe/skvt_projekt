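; Base NPC character that takes hits, attacks and dies, with damage and attacks delegated to a SkvtHealth component.
; Incoming damage feeds the component and plays a punch-hit montage; its OnDeath event ragdolls the mesh, disables movement and destroys the actor after a delay.
; MoveTo sends the NPC by AI to a given spot, where it plays a neck-break montage, snaps to a rotation, then invokes the death handler directly.
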(event `self.SkvtHealth.OnDeath`
  (`PrimitiveComponent.SetSimulatePhysics` (`self.Mesh`) true)
  (`CharacterMovementComponent.DisableMovement` (`self.CharacterMovement`))
  (`KismetSystemLibrary.K2_SetTimerDelegate` (delegate `Destroy`) 10.0))

(event `Destroy`
  (`self.K2_DestroyActor`))

(event `self.ReceiveAnyDamage`
  (params (Damage :type "Float (single-precision)") (DamageType :type "DamageType Object Reference") (InstigatedBy :type "Controller Object Reference") (DamageCauser :type "Actor Object Reference"))
  (`/Game/Skvt/System/Damage/SkvtHealth.ProcessDamage` (`self.SkvtHealth`) Damage)
  (`self.PlayAnimMontage` "/Game/Skvt/Characters/Animations/Attacks/AM_Hit_punch.AM_Hit_punch"))

(event `Attack`
  (`/Game/Skvt/System/Damage/SkvtHealth.Attack` (`self.SkvtHealth`) null null))

(event `MoveTo`
  (params (Location :type "Vector Structure") (Rotation :type "Rotator Structure"))
  (`|AIMoveTo` self Location null
    (:`OnSuccess`
      (`self.PlayAnimMontage` "/Game/Skvt/Characters/Animations/Takedown/Montage_Hit_BreakNeck.Montage_Hit_BreakNeck")
      (`self.K2_SetActorRotation` Rotation)
      (`KismetSystemLibrary.Delay` 1.0)
      (`self.BndEvt__BP_NPC_base_SkvtHealth_K2Node_ComponentBoundEvent_0_OnDeath__DelegateSignature`))))

(fn `UserConstructionScript`)