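; Base NPC Blueprint for behavior-tree-driven characters, bridging pawn sight detection to its AI controller.
; On possession it casts the new controller to AIC_BT_NPCBase and caches the reference.
; PawnSensing forwards every seen pawn to that controller's SeenPlayer, with no player filter or validity check here.
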(event `self.PawnSensing_0.OnSeePawn`
  (params (Pawn :type "Pawn Object Reference"))
  (`/Game/Skvt/Characters/NPC/BehaviorTrees/AIC_BT_NPCBase.SeenPlayer` (`self.ControllerRef`) Pawn))

(event `self.ReceivePossessed`
  (params (NewController :type "Controller Object Reference"))
  (bind _asaic_bt_npcbase (cast `/Game/Skvt/Characters/NPC/BehaviorTrees/AIC_BT_NPCBase` NewController))
  (set `self.ControllerRef` _asaic_bt_npcbase))

(fn `UserConstructionScript`
  (`parent.UserConstructionScript`))